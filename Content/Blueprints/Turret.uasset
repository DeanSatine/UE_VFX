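; Turret actor that fires Bullet actors when its PawnSensing component sees a BP_ThirdPersonCharacter.
; Each sighting spawns a bullet at the Arrow component's transform, gated by CanFire and a FireRate delay.
; It also applies an interpolated look-at rotation toward TargetActor, but to the seen character rather than the turret.
; TargetActor is never assigned here, and Tick only checks its validity.
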(event OnSeePawn(PawnSensing)
  (params (Pawn :type Pawn%20Object%20Reference))
  (bind _asbp_third_person_character (Utilities|Casting|CastToBP_ThirdPersonCharacter Pawn))
  (Transformation|SetActorRotation _asbp_third_person_character (Math|Interpolation|RInterpTo (Transformation|GetActorRotation) (Math|Rotator|FindLookatRotation (Transformation|GetActorLocation) (Transformation|GetActorLocation (Variables|Default|GetTargetActor))) (stale EventTick DeltaSeconds) (Variables|Default|GetTurnSpeed)))
  (if (Variables|Default|GetCanFire)
    (Game|SpawnActorfromClass "/Game/Blueprints/Bullet.Bullet_C" (Transformation|GetWorldTransform (Variables|Default|GetArrow)) "Undefined" "MultiplyWithRoot" 0 0)
    (Variables|Default|SetCanFire false)
    (Utilities|FlowControl|Delay (Variables|Default|GetFireRate))
    (Variables|Default|SetCanFire true)))

(event EventTick
  (params (DeltaSeconds :type Float%20%28single-precision%29))
  (Utilities|IsValid (Variables|Default|GetTargetActor)))

(fn ConstructionScript)