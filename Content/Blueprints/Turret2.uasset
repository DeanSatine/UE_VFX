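; Turret actor that tracks a player-tagged actor inside its sphere trigger and fires lightning effects at it.
; Sphere overlap starts two looping timers, one interpolating the turret top's yaw toward the target and one firing, and clears them on exit.
; Each shot line-traces to the target and, on hitting a player, spawns muzzle, beam and impact particles without applying damage.
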(event OnComponentBeginOverlap(Sphere)
  (params (OverlappedComponent :type Primitive%20Component%20Object%20Reference) (OtherActor :type Actor%20Object%20Reference) (OtherComp :type Primitive%20Component%20Object%20Reference) (OtherBodyIndex :type Integer) (bFromSweep :type Boolean) (SweepResult :type Hit%20Result%20Structure%20%28by%20ref%29))
  ;[0.15 0.15 0.15 0.5] When see player set target
  (Utilities|IsValid OtherActor
    (:Is%20Valid
      (if (Actor|ActorHasTag OtherActor "player")
        (Variables|Default|SetTarget OtherActor)
        (CallFunction|TrackTarget)))))

(event OnComponentEndOverlap(Sphere)
  (params (OverlappedComponent :type Primitive%20Component%20Object%20Reference) (OtherActor :type Actor%20Object%20Reference) (OtherComp :type Primitive%20Component%20Object%20Reference) (OtherBodyIndex :type Integer))
  ;[0.15 0.15 0.15 0.5] When player leaves range stop trackiong
  (Utilities|IsValid OtherActor
    (:Is%20Valid
      (if (Actor|ActorHasTag OtherActor "player")
        (Variables|Default|GetTarget
          (:then
            (Utilities|Time|ClearandInvalidateTimerbyHandle (Variables|Default|GetTimerRef))
            (Utilities|Time|ClearandInvalidateTimerbyHandle (Variables|Default|GetFireTimer)))
          (:else))))))

(event Custom|TrackTarget
  ;[0.15 0.15 0.15 0.5] Rotate Turret
  (bind _returnvalue (Utilities|Time|SetTimerbyEvent (delegate Custom|MoveTurret) 0.05 true))
  (Variables|Default|SetTimerRef _returnvalue)
  (bind _returnvalue_2 (Utilities|Time|SetTimerbyEvent (delegate Custom|ShootTurret) 0.3 true))
  (Variables|Default|SetFireTimer _returnvalue_2))

(event Custom|MoveTurret
  (bind _target (Variables|Default|GetTarget))
  ;[0.15 0.15 0.15 0.5] Rotate Turret
  (Utilities|IsValid _target
    (:Is%20Valid
      (Transformation|SetRelativeRotation (Variables|Default|GetTurretTop) (Math|Rotator|MakeRotator 0.0 0.0 (.yaw (Math|Interpolation|RInterpTo (Variables|/Script/Engine.SceneComponent|GetRelativeRotation (Variables|Default|GetTurretTop)) (Math|Rotator|FindLookatRotation (Transformation|GetActorLocation) (Transformation|GetActorLocation _target)) (Utilities|Time|GetWorldDeltaSeconds) 1e+02))) false false))))

(event Custom|ShootTurret
  ;[0.15 0.15 0.15 0.5] Fireline trace
  (bind (_outhit _returnvalue) (Collision|LineTraceByChannel (+ (Transformation|GetActorLocation) "0.000000,0.000000,80.000000") (Transformation|GetActorLocation (Variables|Default|GetTarget)) "TraceTypeQuery2" true 0 "None"))
  (if _returnvalue
    (if (Actor|ActorHasTag (.HitActor (Collision|BreakHitResult _outhit)) "player")
      (Effects|SpawnEmitterAttached "/Game/FXVarietyPack/Particles/P_ky_shotShockwave.P_ky_shotShockwave" (Variables|Default|GetTurretTop) "FireSocket" "0, 0, 0" "0, 0, 0" "1.000000,1.000000,1.000000" "SnapToTarget")
      (bind _returnvalue_2 (Effects|SpawnEmitterAttached "/Game/FXVarietyPack/Particles/P_ky_lightning1.P_ky_lightning1" (Variables|Default|GetTurretTop) "Bottom"))
      (Effects|Components|ParticleSystem|SetVectorParameter _returnvalue_2 "TargetTest" (Transformation|GetActorLocation (Variables|Default|GetTarget)))
      (Effects|SpawnEmitteratLocation "/Game/FXVarietyPack/Particles/P_ky_hit2.P_ky_hit2" (.ImpactPoint (Collision|BreakHitResult _outhit))))))

(fn ConstructionScript)